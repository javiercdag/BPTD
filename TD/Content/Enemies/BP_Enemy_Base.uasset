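; Base enemy character Blueprint that provides shared aggro, patrol, movement and attack functions.
; Attack is a placeholder that uncrouches, prints a debug message, waits, then calls the OnAttackEnd dispatcher to signal completion.
; Aggro and SetAggro update the aggro flag, and GetPatrolRoute exposes the assigned route.
; SetMovementSpeed maps an idle-to-sprint movement state onto the character's max walk speed.
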(event `Attack`
  (`self.UnCrouch`)
  (`KismetSystemLibrary.PrintText` "Attacking")
  (`KismetSystemLibrary.Delay` 4.0)
  (`self.OnAttackEnd`))

(event `Aggro`
  (set `self.IsAggroed` true))

(fn `GetPatrolRoute`
  (returns (PatrolRoute :type "/Game/Enemies/AI/BP_PatrolRoute Object Reference"))
  (return (`self.PatrolRoute`)))

(fn `SetAggro`
  (params (IsAggroed :type Boolean))
  (returns (Aggro :type Boolean))
  (bind _output_get (set `self.IsAggroed` IsAggroed))
  (return _output_get))

(fn `SetMovementSpeed`
  (params (MovementSpeed :type "/Game/Enemies/AI/Enums/E_MovementSpeed Enum" :default "NewEnumerator0"))
  (returns (Speed :type "Float (double-precision)"))
  (bind _output_get (set `CharacterMovementComponent.MaxWalkSpeed` (select `/Game/Enemies/AI/Enums/E_MovementSpeed` MovementSpeed :`NewEnumerator1` 100.0 :`NewEnumerator2` 300.0 :`NewEnumerator3` 500.0 :!type "Float (single-precision)") (`self.CharacterMovement`)))
  (return _output_get))

(fn `UserConstructionScript`)