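; BP_PatrolRoute defines an enemy AI patrol path from the points of its PatrolRoute spline.
; GetSplinePointAsWorldPosition returns the world location of the current patrol point.
; IncrementPatrolRoute steps the current index by Direction, which flips at the last and first points so the route is traversed back and forth rather than looped.
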(event `IncrementPatrolRoute`
  (bind _output_get (set `self.CurrentPatrolPointIndex` (+ (`self.CurrentPatrolPointIndex`) (`self.Direction`))))
  (if (== _output_get (- (`SplineComponent.GetNumberOfSplinePoints` (`self.PatrolRoute`)) 1))
    (set `self.Direction` -1)
    (elif (== (`self.CurrentPatrolPointIndex`) 0)
      (set `self.Direction` 1))))

(fn `GetSplinePointAsWorldPosition`
  (returns (Location :type "Vector Structure"))
  (return (`SplineComponent.GetLocationAtSplinePoint` (`self.PatrolRoute`) (`self.CurrentPatrolPointIndex`) "World")))

(fn `UserConstructionScript`)